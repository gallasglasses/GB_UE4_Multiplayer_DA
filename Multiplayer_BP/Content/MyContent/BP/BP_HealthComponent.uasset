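; Health component that tracks an actor's health, starting at max, and broadcasts health-change and death events.
; Server_TakeDamage applies damage through Multicast_SetHealth, then either fires OnDeath or, with AutoHeal on, restarts a delayed looping HealUpdate timer that stops at full health.
; Healing and TryToAddHealth use the non-multicast SetHealth, with pickup-style adds refused when dead or full.
; OnRep_Health only prints the value.
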(event Custom|Multicast_SetHealth
  (params (NewHealth :type Float%20%28single-precision%29))
  ;[1 1 1] Multicast SetHealth
  (bind _output_get (Variables|Health|SetHealth (Math|Float|Clamp(Float) NewHealth 0.0 (Variables|Health|GetMaxHealth))))
  (Default|CallOnHealthChanged _output_get))

(event Custom|Server_TakeDamage
  (params (Damage :type Float%20%28single-precision%29))
  ;[1 1 1] Server TakeDamage
  (bind _bisdead (CallFunction|IsDead))
  (if (not (or (<= Damage 0.0) _bisdead))
    (CallFunction|MulticastSetHealth (- (Variables|Health|GetHealth) Damage))
    (Utilities|Time|ClearandInvalidateTimerbyHandle (Variables|Default|GetHealTimerHandle))
    (bind _bisdead_2 (CallFunction|IsDead))
    (if _bisdead_2
      (Default|CallOnDeath)
      (elif (Variables|Heal|GetAutoHeal)
        (bind _returnvalue (Utilities|Time|SetTimerbyFunctionName self "HealUpdate" (Variables|Heal|GetHealUpdateTime) true (Variables|Heal|GetHealDelay)))
        (Variables|Default|SetHealTimerHandle _returnvalue)))))

(event EventBeginPlay
  (CallFunction|SetHealth (Variables|Health|GetMaxHealth)))

(fn GetHealth
  (return (Variables|Health|GetHealth)))

(fn OnRepHealth
  (Development|PrintString (Utilities|String|ToString(Float) (Variables|Health|GetHealth))))

(fn GetHealthPercent
  (return (/ (Variables|Health|GetHealth) (Variables|Health|GetMaxHealth))))

(fn IsDead
  (return (Math|Float|NearlyEqual(Float) (Variables|Health|GetHealth) 0.0 1e-06)))

(fn HealUpdate
  (CallFunction|SetHealth (+ (Variables|Health|GetHealth) (Variables|Heal|GetHealModifier)))
  (bind _bishealthfull (CallFunction|IsHealthFull))
  (if _bishealthfull
    (Utilities|Time|ClearandInvalidateTimerbyHandle (Variables|Default|GetHealTimerHandle))))

(fn SetHealth
  (params (NewHealth :type Float%20%28single-precision%29))
  (bind _output_get (Variables|Health|SetHealth (Math|Float|Clamp(Float) NewHealth 0.0 (Variables|Health|GetMaxHealth))))
  (Default|CallOnHealthChanged _output_get))

(fn IsHealthFull
  (return (Math|Float|NearlyEqual(Float) (Variables|Health|GetHealth) (Variables|Health|GetMaxHealth) 1e-06)))

(fn TrytoAddHealth
  (params (HealthAmount :type Float%20%28single-precision%29))
  (bind _bisdead (CallFunction|IsDead))
  (bind _bishealthfull (CallFunction|IsHealthFull))
  (if (or _bishealthfull _bisdead)
    (return false)
    (else
      (CallFunction|SetHealth (+ HealthAmount (Variables|Health|GetHealth)))
      (return true))))