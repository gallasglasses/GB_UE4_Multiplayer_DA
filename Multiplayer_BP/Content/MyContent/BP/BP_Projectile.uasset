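; BP_Projectile is a multiplayer projectile that damages characters and explodes on impact.
; On the server, Tick moves it along its forward vector without sweeping, and sphere overlaps drive hit handling.
; Hits ignore the owner and other projectiles, damage any BP_MultiplayerCharacter, multicast an explosion effect, then destroy the projectile.
; A lifetime timer started on BeginPlay also routes to the server destroy event.
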(event OnComponentBeginOverlap(SphereCollision)
  (params (OverlappedComponent :type Primitive%20Component%20Object%20Reference) (OtherActor :type Actor%20Object%20Reference) (OtherComp :type Primitive%20Component%20Object%20Reference) (OtherBodyIndex :type Integer) (bFromSweep :type Boolean) (SweepResult :type Hit%20Result%20Structure%20%28by%20ref%29))
  (if (Networking|IsServer)
    (CallFunction|ServeronProjectileHit OtherActor (Transformation|GetActorLocation))))

(event Custom|LifeEnded
  (CallFunction|ServerLifeEnded))

(event Custom|Server_LifeEnded
  (Actor|DestroyActor))

(event Custom|Server_Move
  (params (DeltaTime :type Float%20%28single-precision%29))
  (Transformation|SetActorLocation (+ (* (Transformation|GetActorForwardVector) (* DeltaTime (Variables|Float|GetSpeed))) (Transformation|GetActorLocation)) false false))

(event Custom|Server_OnProjectileHit
  (params (OtherActor :type Actor%20Object%20Reference) (Location :type Vector))
  (if (!= OtherActor (Components|GetOwner))
    (bind _asbp_multiplayer_character (Utilities|Casting|CastToBP_MultiplayerCharacter OtherActor)
      (:then
        (Default|MakeDamage _asbp_multiplayer_character (Variables|Float|GetDamage)))
      (:CastFailed
        (Utilities|Casting|CastToBP_Projectile OtherActor
          (:CastFailed
            _))))
    (CallFunction|MulticastHitEffect Location)
    (CallFunction|ServerLifeEnded)))

(event Custom|SpawnHitEffect
  (params (HitLocation :type Vector))
  (Effects|SpawnEmitteratLocation "/Game/StarterContent/Particles/P_Explosion.P_Explosion" HitLocation))

(event Custom|Multicast_HitEffect
  (params (HitLocation :type Vector))
  (CallFunction|SpawnHitEffect HitLocation))

(event EventBeginPlay
  (Utilities|Time|SetTimerbyEvent (delegate Custom|LifeEnded) (Variables|Float|GetLifeTime)))

(event Collision|EventActorBeginOverlap
  (params (OtherActor :type Actor%20Object%20Reference)))

(event EventTick
  (params (DeltaSeconds :type Float%20%28single-precision%29))
  (if (Networking|IsServer)
    (CallFunction|ServerMove DeltaSeconds)))

(fn ConstructionScript)